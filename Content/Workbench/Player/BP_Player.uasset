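; Player character Blueprint that handles interaction, player switching and death.
; Input actions call FindNearestActor, which filters capsule overlaps by interface and compares horizontal distance, favoring larger values despite its name, then messages the result through BPI_Interact or BPI_Rkey.
; Any damage or DeathEvent updates the GameInstance death count once, ragdolls the mesh, then reloads the stage level after delays including the loading display.
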(event `InputAction|PlayerChange`
  (params (Key :type "Key Structure"))
  (:`Pressed`
    (`self.PlayerChange`)))

(event `InputAction|Interacted`
  (params (Key :type "Key Structure"))
  (:`Pressed`
    (`self.Interact`)))

(event `self.ReceiveAnyDamage`
  (params (Damage :type "Float (single-precision)") (DamageType :type "DamageType Object Reference") (InstigatedBy :type "Controller Object Reference") (DamageCauser :type "Actor Object Reference"))
  (bind _mesh (`self.Mesh`))
  (bind _asbp_game_instance (cast `/Game/Workbench/BP_GameInstance` (`GameplayStatics.GetGameInstance`) :!pure true))
  ;[1 1 1] プレイヤーの死
  (`|ExecutionSequence` :!label _label
    (:`then_0`
      (`/Engine/EditorBlueprintResources/StandardMacros.DoOnce` false
        (:`Completed`
          (set `self.Game InstanceRef` _asbp_game_instance)
          (`/Game/Workbench/BP_GameInstance.SetDeathCount` _asbp_game_instance))))
    (:`then_1`
      (`CharacterMovementComponent.DisableMovement` (`self.CharacterMovement`))
      (`PrimitiveComponent.SetCollisionProfileName` _mesh "Ragdoll" true)
      (`PrimitiveComponent.SetSimulatePhysics` _mesh true))
    (:`then_2`
      ;;[1 1 1] ロードしなおし(オブジェクト復元)
      (`KismetSystemLibrary.Delay` 2.0)
      (bind _loadingtime (`/Game/Workbench/BP_GameInstance.LoadingDisplay` (`self.Game InstanceRef`)))
      (`KismetSystemLibrary.Delay` _loadingtime)
      (bind _output_get (set `self.Level Name` (`/Game/Workbench/BP_GameInstance.Stage` (`self.Game InstanceRef`))))
      (`GameplayStatics.OpenLevel` _output_get))))

(event `DeathEvent`
  ;[1 1 1] プレイヤーの死
  (goto _label))

(fn `FindNearestActor`
  (params (Interface :type "Interface Class Reference"))
  (returns (ReturnValue :type "Actor Object Reference"))
  (set `self.TempDistance` 0.0)
  (set `self.Overlapping Actors` (`PrimitiveComponent.GetOverlappingActors` (`self.CapsuleComponent`) "/Script/Engine.Actor"))
  (if (`KismetArrayLibrary.Array_IsValidIndex` (`self.Overlapping Actors`))
    (for (_array_element _array_index) (`self.Overlapping Actors`)
      (if (`KismetSystemLibrary.DoesImplementInterface` _array_element Interface)
        (bind _returnvalue (`self.GetHorizontalDistanceTo` self _array_element))
        (if (< (`self.TempDistance`) _returnvalue)
          (set `self.TempDistance` _returnvalue)
          (set `self.Array Index` _array_index))))
    (return (`|GetArrayItem` (`self.Overlapping Actors`) (`self.Array Index`)))
    (else
      (return null))))

(fn `Interact`
  (bind _returnvalue (`self.FindNearestActor` "/Game/Workbench/BliePrint/1F/BPI_Interact.BPI_Interact_C"))
  (`/Engine/EditorBlueprintResources/StandardMacros.IsValid` _returnvalue
    (:`Is Valid`
      (message `/Game/Workbench/BliePrint/1F/BPI_Interact.HasInteracted` _returnvalue))))

(fn `OffInteract`
  (bind _returnvalue (`self.FindNearestActor` "/Game/Workbench/BliePrint/1F/BPI_Interact.BPI_Interact_C"))
  (`/Engine/EditorBlueprintResources/StandardMacros.IsValid` _returnvalue
    (:`Is Valid`
      (message `/Game/Workbench/BliePrint/1F/BPI_Interact.OffInteracted` _returnvalue))))

(fn `PlayerChange`
  (bind _returnvalue (`self.FindNearestActor` "/Game/Workbench/BliePrint/1F/BPI_Rkey.BPI_Rkey_C"))
  (`/Engine/EditorBlueprintResources/StandardMacros.IsValid` _returnvalue
    (:`Is Valid`
      (message `/Game/Workbench/BliePrint/1F/BPI_Rkey.ChangePlayer` _returnvalue))))

(fn `UserConstructionScript`)