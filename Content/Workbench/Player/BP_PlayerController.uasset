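; Player controller that handles movement, mouse look, jump, timeline-eased sprint, self-destruct and the back-to-title menu.
; When the game mode's CameraChenge flag is set, movement uses world-direction arrays indexed by GameInstance camera flags; otherwise it follows control rotation.
; BackTitle shows a widget created at BeginPlay, disables movement and blocks look input.
; A hidden command, gated by holding 1, increments and saves DeathCount; an overlap-trigger check is left unconnected.
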(event `self.ReceiveBeginPlay`
  (bind _returnvalue (`GameplayStatics.GetPlayerCameraManager` 0))
  (bind _returnvalue_2 (`|CreateWidget` "/Game/Workbench/BliePrint/StartAndEnd/WBP_BackTitle.WBP_BackTitle_C"))
  (set `self.BackTitleRef` _returnvalue_2)
  (set `CharacterMovementComponent.MaxWalkSpeed` (`self.WalkSpeed`) (`Character.CharacterMovement` (cast `Character` (`self.K2_GetPawn`) :!pure true)))
  ;[1 1 1] カメラ回転制御
  (set `PlayerCameraManager.ViewPitchMin` (`self.View Pitch Min`) _returnvalue)
  (set `PlayerCameraManager.ViewPitchMax` (`self.View Pitch Max`) _returnvalue))

(event `InputAction|DeathKey`
  (params (Key :type "Key Structure"))
  ;[1 1 1] 自爆(グレイマンのみ)
  (:`Pressed`
    (`/Game/Workbench/Player/BP_Player.DeathEvent` (cast `/Game/Workbench/Player/BP_Player` (`self.K2_GetPawn`) :!pure true))))

(event `InputAction|Sprint`
  (params (Key :type "Key Structure"))
  ;[1 1 1] ダッシュ
  (:`Pressed`
    (bind (_direction `_新規track_0`) (`Timeline|ChangeSpeed` :!label _label)
      (:`Update`
        (set `CharacterMovementComponent.MaxWalkSpeed` (`KismetMathLibrary.Lerp` (`self.WalkSpeed`) (`self.SprintSpeed`) `_新規track_0`) (`Character.CharacterMovement` (cast `Character` (`self.K2_GetPawn`) :!pure true))))))
  (:`Released`
    (goto _label :!via `Reverse`)))

(event `InputAction|Jump`
  (params (Key :type "Key Structure"))
  (bind _ascharacter (cast `Character` (`self.K2_GetPawn`) :!pure true))
  ;[1 1 1] ジャンプ(1段階ジャンプのみに設定、途中で切り替えるのもあり)
  (:`Pressed`
    (`Character.Jump` _ascharacter)
    (`self.JumpEvent`))
  (:`Released`
    (`Character.StopJumping` _ascharacter)))

(event `InputAxis|MoveForward`
  (params (AxisValue :type "Float (single-precision)"))
  (bind _returnvalue (`self.K2_GetPawn`))
  (bind (_returnvalue_roll _returnvalue_pitch _returnvalue_yaw) (`KismetMathLibrary.BreakRotator` (`Pawn.GetControlRotation` _returnvalue)))
  (bind _asbp_game_instance (cast `/Game/Workbench/BP_GameInstance` (`GameplayStatics.GetGameInstance`) :!pure true))
  (bind _cameraforwarddirectionpositive (`/Game/Workbench/BP_GameInstance.CameraForwardDirectionPositive` _asbp_game_instance))
  ;[1 1 1] 前後移動(視点が移動するカメラに合わせてカメラから見た前後移動をする)
  (if (`/Game/Workbench/BP_Gamemode.CameraChenge` (cast `/Game/Workbench/BP_Gamemode` (`GameplayStatics.GetGameMode`) :!pure true))
    (if (`/Game/Workbench/BP_GameInstance.CameraForwardDirectionX` _asbp_game_instance)
      (if _cameraforwarddirectionpositive
        (set `self.ForwardBackDirectionIndex` 0)
        (else
          (set `self.ForwardBackDirectionIndex` 1)))
      (elif _cameraforwarddirectionpositive
        (set `self.ForwardBackDirectionIndex` 2)
        (else
          (set `self.ForwardBackDirectionIndex` 3))))
    (`Pawn.AddMovementInput` _returnvalue (`|GetArrayItem` (`self.ForwardBackDirection`) (`self.ForwardBackDirectionIndex`)) AxisValue false)
    (else
      (`Pawn.AddMovementInput` _returnvalue (`KismetMathLibrary.GetForwardVector` (`KismetMathLibrary.MakeRotator` _returnvalue_roll _returnvalue_pitch _returnvalue_yaw)) AxisValue false)
      (set `self.ForwardScale` AxisValue)
      (`self.MoveForward`))))

(event `InputAxis|LookUp/Down`
  (params (AxisValue :type "Float (single-precision)"))
  ;[1 1 1] カメラ移動
  (if (not (`self.DisplayUI`))
    (`Pawn.AddControllerPitchInput` (`self.K2_GetPawn`) (* AxisValue (`self.MouseSensitibityY`)))))

(event `InputAxis|MoveRight`
  (params (AxisValue :type "Float (single-precision)"))
  (bind _returnvalue (`self.K2_GetPawn`))
  (bind (_returnvalue_roll _returnvalue_pitch _returnvalue_yaw) (`KismetMathLibrary.BreakRotator` (`Pawn.GetControlRotation` _returnvalue)))
  (bind _asbp_game_instance (cast `/Game/Workbench/BP_GameInstance` (`GameplayStatics.GetGameInstance`) :!pure true))
  (bind _camerarightdirectionpositive (`/Game/Workbench/BP_GameInstance.CameraRightDirectionPositive` _asbp_game_instance))
  ;[1 1 1] 前後移動(視点が移動するカメラに合わせてカメラから見た前後移動をする)
  (if (`/Game/Workbench/BP_Gamemode.CameraChenge` (cast `/Game/Workbench/BP_Gamemode` (`GameplayStatics.GetGameMode`) :!pure true))
    (if (`/Game/Workbench/BP_GameInstance.CameraRightDirectionX` _asbp_game_instance)
      (if _camerarightdirectionpositive
        (set `self.RightLeftDirectionIndex` 0)
        (else
          (set `self.RightLeftDirectionIndex` 1)))
      (elif _camerarightdirectionpositive
        (set `self.RightLeftDirectionIndex` 2)
        (else
          (set `self.RightLeftDirectionIndex` 3))))
    (`Pawn.AddMovementInput` _returnvalue (`|GetArrayItem` (`self.RightLeftDirection`) (`self.RightLeftDirectionIndex`)) AxisValue false)
    (else
      (`Pawn.AddMovementInput` _returnvalue (`KismetMathLibrary.GetRightVector` (`KismetMathLibrary.MakeRotator` _returnvalue_roll _returnvalue_pitch _returnvalue_yaw)) AxisValue false)
      (set `self.RightScale` AxisValue)
      (`self.MoveRight`))))

(event `InputAxis|LookRight/Left`
  (params (AxisValue :type "Float (single-precision)"))
  ;[1 1 1] カメラ移動
  (if (not (`self.DisplayUI`))
    (`Pawn.AddControllerYawInput` (`self.K2_GetPawn`) (* AxisValue (`self.MouseSensitibityX`)))))

(event `InputAction|PlayerChange`
  (params (Key :type "Key Structure")))

(event `Key|One`
  (params (Key :type "Key Structure"))
  (:`Pressed`
    (set `self.HiddenCommand` true))
  (:`Released`
    (set `self.HiddenCommand` false)))

(event `InputAction|Hidden Command`
  (params (Key :type "Key Structure"))
  (bind _savedata (`/Game/Workbench/BP_GameInstance.SaveData` (cast `/Game/Workbench/BP_GameInstance` (`GameplayStatics.GetGameInstance`) :!pure true)))
  (:`Pressed`
    (if (`self.HiddenCommand`)
      (bind _result (`/Engine/EditorBlueprintResources/StandardMacros.IncrementInt` (`/Game/Workbench/BP_SaveGame.DeathCount` _savedata))
        (:`  `
          (bind _output_get (set `/Game/Workbench/BP_SaveGame.DeathCount` _result _savedata))
          (`GameplayStatics.SaveGameToSlot` _savedata (`/Game/Workbench/BP_SaveGame.Slot Name` _savedata))
          (`KismetSystemLibrary.PrintString` (`KismetStringLibrary.Conv_IntToString` _output_get)))))))

(event `InputAction|BackTitle`
  (params (Key :type "Key Structure"))
  (:`Pressed`
    (`CharacterMovementComponent.DisableMovement` (`Character.CharacterMovement` (cast `Character` (`self.K2_GetPawn`) :!pure true)))
    (set `self.bShowMouseCursor` true)
    (`UserWidget.AddToViewport` (`self.BackTitleRef`) 0)
    (set `self.DisplayUI` true)))

(fn `UserConstructionScript`)