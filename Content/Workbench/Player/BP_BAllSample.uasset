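; BP_BAllSample is a player-controlled rolling ball that moves and jumps through physics.
; Forward and right axis inputs apply torque scaled by RollTorque to the Ball component to roll it.
; Jump applies an upward impulse when CanJump is set, then clears the flag until any Hit event restores it, with no check on surface direction.
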(event `InputAxis|MoveRight`
  (params (AxisValue :type "Float (single-precision)"))
  (`PrimitiveComponent.AddTorqueInRadians` (`self.Ball`) (`KismetMathLibrary.MakeVector` (* (`self.RollTorque`) AxisValue -1.0)) "None" false))

(event `InputAxis|MoveForward`
  (params (AxisValue :type "Float (single-precision)"))
  (`PrimitiveComponent.AddTorqueInRadians` (`self.Ball`) (`KismetMathLibrary.MakeVector` 0.0 (* (`self.RollTorque`) AxisValue)) "None" false))

(event `InputAction|Jump`
  (params (Key :type "Key Structure"))
  (:`Pressed`
    (if (`self.CanJump`)
      (`PrimitiveComponent.AddImpulse` (`self.Ball`) (`KismetMathLibrary.MakeVector` 0.0 0.0 (`self.JumpImpulse`)) "None" false)
      (set `self.CanJump` false))))

(event `self.ReceiveHit`
  (params (MyComp :type "PrimitiveComponent Object Reference") (Other :type "Actor Object Reference") (OtherComp :type "PrimitiveComponent Object Reference") (bSelfMoved :type Boolean) (HitLocation :type "Vector Structure") (HitNormal :type "Vector Structure") (NormalImpulse :type "Vector Structure") (Hit :type "HitResult Structure (by ref)"))
  (set `self.CanJump` true))

(fn `UserConstructionScript`)