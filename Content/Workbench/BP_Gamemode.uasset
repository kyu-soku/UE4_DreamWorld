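; Game mode Blueprint that provides player respawning for the first player when its pawn is destroyed.
; RespawnEvent binds RespawnPlayer to the pawn's OnDestroyed, which spawns a new BP_Player at a player start, possesses it and rebinds for the next death.
; BeginPlay only clears the BPBall reference; the initial RespawnEvent call is unwired, so nothing in this graph starts the respawn cycle.
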(event `self.ReceiveBeginPlay`
  (set `self.BP_Ball` null))

(event `RespawnEvent`
  ;[1 1 1] プレイヤーリスポーン
  (add `self.OnDestroyed` (`GameplayStatics.GetPlayerPawn` 0) (delegate `RespawnPlayer`)))

(event `RespawnPlayer` :!signature `self.OnDestroyed`
  (params (DestroyedActor :type "Actor Object Reference"))
  ;[1 1 1] プレイヤーリスポーン
  (bind _returnvalue (`|SpawnActorFromClass` "/Game/Workbench/Player/BP_Player.BP_Player_C" (`self.GetTransform` (`self.K2_FindPlayerStart` null)) "Undefined" "OverrideRootScale" null null))
  (`Controller.Possess` (`GameplayStatics.GetPlayerController` 0) _returnvalue)
  (`self.RespawnEvent`))

(fn `UserConstructionScript`)