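; BP_Lane_Acceleration is a lane trigger that spins the game's ball to speed it along one axis while active.
; Overlapping the Trigger plays the Accele timeline, and ending the overlap stops it.
; Each timeline update scales Torque by the Accelex curve and applies it to the Physics component of BPBall from BP_Gamemode.
; The DirectionYYXX selector chooses positive or negative X or Y as the torque axis.
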(event `self.Trigger.OnComponentBeginOverlap`
  (params (OverlappedComponent :type "PrimitiveComponent Object Reference") (OtherActor :type "Actor Object Reference") (OtherComp :type "PrimitiveComponent Object Reference") (OtherBodyIndex :type Integer) (bFromSweep :type Boolean) (SweepResult :type "HitResult Structure (by ref)"))
  (bind _torque (`self.Torque`))
  (bind (_direction _accelex) (`Timeline|accele` :!label _label)
    (:`Update`
      (`PrimitiveComponent.AddTorqueInRadians` (`/Game/Workbench/BliePrint/2F/BP_BallPhysics.physics` (`/Game/Workbench/BP_Gamemode.BP_Ball` (cast `/Game/Workbench/BP_Gamemode` (`GameplayStatics.GetGameMode`) :!pure true))) (select `int` (`self.Direction(-Y,Y,X,-X)`) :`0` (`KismetMathLibrary.MakeVector` (* _accelex _torque)) :`1` (`KismetMathLibrary.MakeVector` (* _accelex _torque -1.0)) :`2` (`KismetMathLibrary.MakeVector` 0.0 (* _accelex _torque)) :`3` (`KismetMathLibrary.MakeVector` 0.0 (* _accelex _torque -1.0))) "None" false))))

(event `self.Trigger.OnComponentEndOverlap`
  (params (OverlappedComponent :type "PrimitiveComponent Object Reference") (OtherActor :type "Actor Object Reference") (OtherComp :type "PrimitiveComponent Object Reference") (OtherBodyIndex :type Integer))
  (goto _label :!via `Stop`))

(fn `UserConstructionScript`)