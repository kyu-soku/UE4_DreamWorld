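; An interactable switch that rotates or moves referenced lane pieces: a corner, short corner, set of lines or set of change-lines.
; BeginPlay copies CoolTime into each valid piece's rotate or move time, keeping animation and lockout in sync.
; HasInteracted picks the target by boolean flags, advancing rotation 90 degrees per use or firing MoveEvent on change-lines.
; A DoOnce plus Delay blocks re-triggering during the cooldown while the switch material is swapped.
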(event `self.ReceiveBeginPlay`
  (bind _bp_coner (`self.BP_Coner`))
  (bind _bp_shortconer (`self.BP_ShortConer`))
  (`/Engine/EditorBlueprintResources/StandardMacros.IsValid` _bp_coner
    (:`Is Valid`
      (set `/Game/Workbench/BliePrint/2F/BP_ConerLane.RotateTime` (`self.CoolTime`) _bp_coner))
    (:`Is Not Valid`
      _))
  (`/Engine/EditorBlueprintResources/StandardMacros.IsValid` _bp_shortconer
    (:`Is Valid`
      (set `/Game/Workbench/BliePrint/2F/BP_ShortConerLane.RotateTime` (`self.CoolTime`) _bp_shortconer))
    (:`Is Not Valid`
      _))
  (for _array_element (`self.BP_ChangeLine`)
    (`/Engine/EditorBlueprintResources/StandardMacros.IsValid` _array_element
      (:`Is Valid`
        (set `/Game/Workbench/BliePrint/2F/BP_ChangeLane.MoveTime` (`self.CoolTime`) _array_element))))
  (for _array_element_2 (`self.BP_LineRef`)
    (`/Engine/EditorBlueprintResources/StandardMacros.IsValid` _array_element_2
      (:`Is Valid`
        (set `/Game/Workbench/BliePrint/2F/BP_Lane.RotateTime` (`self.CoolTime`) _array_element_2)))))

(event `/Game/Workbench/BliePrint/1F/BPI_Interact.HasInteracted`
  (bind _rotatex (`self.RotateX`))
  (bind _rotatex_2 (`self.RotateX`))
  (bind _rotatex_3 (`self.RotateX`))
  (if (`self.ShortConer`)
    (`/Engine/EditorBlueprintResources/StandardMacros.DoOnce` false :!label _label
      (:`Completed`
        (`PrimitiveComponent.SetMaterial` (`self.Switch`) 1 "/Game/Workbench/Material/M_Glassbikkuri.M_Glassbikkuri")
        (`/Game/Workbench/BliePrint/2F/BP_ShortConerLane.RotationX` (`self.BP_ShortConer`) _rotatex_3)
        (set `self.RotateX` (+ _rotatex_3 90.0))
        (`KismetSystemLibrary.Delay` (`self.CoolTime`))
        (`PrimitiveComponent.SetMaterial` (`self.Switch`) 1 "/Game/Workbench/Material/M_bikkuri.M_bikkuri")
        (goto _label :!via `Reset`)))
    (elif (`self.Line`)
      (`/Engine/EditorBlueprintResources/StandardMacros.DoOnce` false :!label _label_2
        (:`Completed`
          (`PrimitiveComponent.SetMaterial` (`self.Switch`) 1 "/Game/Workbench/Material/M_Glassbikkuri.M_Glassbikkuri")
          (for _array_element (`self.BP_LineRef`)
            (`/Game/Workbench/BliePrint/2F/BP_Lane.RotationtX` _array_element _rotatex_2))
          (set `self.RotateX` (+ _rotatex_2 90.0))
          (`KismetSystemLibrary.Delay` (`self.CoolTime`))
          (`PrimitiveComponent.SetMaterial` (`self.Switch`) 1 "/Game/Workbench/Material/M_bikkuri.M_bikkuri")
          (goto _label_2 :!via `Reset`)))
      (elif (`self.ChangeLane`)
        (`/Engine/EditorBlueprintResources/StandardMacros.DoOnce` false :!label _label_3
          (:`Completed`
            (`PrimitiveComponent.SetMaterial` (`self.Switch`) 1 "/Game/Workbench/Material/M_Glassbikkuri.M_Glassbikkuri")
            (for _array_element_2 (`self.BP_ChangeLine`)
              (`/Game/Workbench/BliePrint/2F/BP_ChangeLane.MoveEvent` _array_element_2))
            (`KismetSystemLibrary.Delay` (`self.CoolTime`))
            (`PrimitiveComponent.SetMaterial` (`self.Switch`) 1 "/Game/Workbench/Material/M_bikkuri.M_bikkuri")
            (goto _label_3 :!via `Reset`)))
        (else
          (`/Engine/EditorBlueprintResources/StandardMacros.DoOnce` false :!label _label_4
            (:`Completed`
              (`PrimitiveComponent.SetMaterial` (`self.Switch`) 1 "/Game/Workbench/Material/M_Glassbikkuri.M_Glassbikkuri")
              (`/Game/Workbench/BliePrint/2F/BP_ConerLane.RotationX` (`self.BP_Coner`) _rotatex)
              (set `self.RotateX` (+ _rotatex 90.0))
              (`KismetSystemLibrary.Delay` (`self.CoolTime`))
              (`PrimitiveComponent.SetMaterial` (`self.Switch`) 1 "/Game/Workbench/Material/M_bikkuri.M_bikkuri")
              (goto _label_4 :!via `Reset`))))))))

(fn `UserConstructionScript`)