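; BP_ChangeLane is a Blueprint that slides its ShortConer component along local Y, apparently to switch lanes.
; BeginPlay sets the offset's sign from the Negative flag.
; MoveY plays the Move timeline at a rate derived from MoveTime, lerping the component from zero to that offset.
; Move-Y reverses the timeline, but both FlipFlop outputs in MoveEvent call MoveY, so MoveEvent never reverses it.
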(event `self.ReceiveBeginPlay`
  (if (`self.Negative`)
    (set `self.Movement` -200.0)
    (else
      (set `self.Movement` 200.0))))

(event `MoveY`
  (`TimelineComponent.SetPlayRate` (`self.Move`) (/ 1.0 (`self.MoveTime`)))
  (bind (_direction _move) (`Timeline|Move` :!label _label)
    (:`Update`
      (`SceneComponent.K2_SetRelativeLocation` (`self.ShortConer`) (`KismetMathLibrary.MakeVector` 0.0 (`KismetMathLibrary.Lerp` 0.0 (`self.Movement`) _move) 0.1) false false))))

(event `Move-Y`
  (goto _label :!via `Reverse`))

(event `MoveEvent`
  (`/Engine/EditorBlueprintResources/StandardMacros.FlipFlop`
    (:`A`
      (`self.MoveY`))
    (:`B`
      (`self.Move-Y`))))

(fn `UserConstructionScript`)