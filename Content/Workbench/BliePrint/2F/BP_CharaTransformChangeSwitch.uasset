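; Floor-switch actor that moves a referenced other player to preset transforms each time it is fully pressed.
; Overlapping the trigger plays a timeline that lowers the switch mesh, and leaving reverses it.
; When the timeline finishes at 1, a configurable count of two, three or four selects the cycle through the PlayerTransform array, using a FlipFlop or a modulo counter, with an error print otherwise.
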(event `self.ReceiveBeginPlay`)

(event `self.Trigger.OnComponentBeginOverlap`
  (params (OverlappedComponent :type "PrimitiveComponent Object Reference") (OtherActor :type "Actor Object Reference") (OtherComp :type "PrimitiveComponent Object Reference") (OtherBodyIndex :type Integer) (bFromSweep :type Boolean) (SweepResult :type "HitResult Structure (by ref)"))
  (bind _howmanytimes_2or3or4_ (`self.HowManyTimes(2or3or4)`))
  (bind (_direction _onoff) (`Timeline|ONOFF` :!label _label)
    (:`Update`
      (`SceneComponent.K2_SetRelativeLocation` (`self.Switch`) (`KismetMathLibrary.VLerp` (0.0 0.0 12.1) (0.0 0.0 0.1) _onoff) false false))
    (:`Finished`
      (if (== _onoff 1.0)
        (if (== _howmanytimes_2or3or4_ 2)
          (`self.Transform(TwoTimes)`)
          (elif (== _howmanytimes_2or3or4_ 3)
            (`self.Transform(ThreeTimes)`)
            (elif (== _howmanytimes_2or3or4_ 4)
              (`self.Transform(fourTimes)`)
              (else
                (`KismetSystemLibrary.PrintString` "エラー")))))))))

(event `self.Trigger.OnComponentEndOverlap`
  (params (OverlappedComponent :type "PrimitiveComponent Object Reference") (OtherActor :type "Actor Object Reference") (OtherComp :type "PrimitiveComponent Object Reference") (OtherBodyIndex :type Integer))
  (goto _label :!via `Reverse`))

(event `Transform(TwoTimes)`
  (`/Engine/EditorBlueprintResources/StandardMacros.FlipFlop`
    (:`A`
      (`self.K2_SetActorTransform` (`self.otherPlaerRef`) (`|GetArrayItem` (`self.PlayerTransform`)) false false))
    (:`B`
      (`self.K2_SetActorTransform` (`self.otherPlaerRef`) (`|GetArrayItem` (`self.PlayerTransform`) 1) false false))))

(event `Transform(ThreeTimes)`
  (bind _returnvalue (mod (`self.Count`) 3))
  (if (== _returnvalue 0)
    (`self.K2_SetActorTransform` (`self.otherPlaerRef`) (`|GetArrayItem` (`self.PlayerTransform`)) false false)
    (set `self.Count` (+ (`self.Count`) 1) :!label _label_2)
    (elif (== _returnvalue 1)
      (`self.K2_SetActorTransform` (`self.otherPlaerRef`) (`|GetArrayItem` (`self.PlayerTransform`) 1) false false)
      (goto _label_2)
      (elif (== _returnvalue 2)
        (`self.K2_SetActorTransform` (`self.otherPlaerRef`) (`|GetArrayItem` (`self.PlayerTransform`) 2) false false)
        (goto _label_2)))))

(event `Transform(fourTimes)`
  (bind _returnvalue (mod (`self.Count`) 4))
  (if (== _returnvalue 0)
    (`self.K2_SetActorTransform` (`self.otherPlaerRef`) (`|GetArrayItem` (`self.PlayerTransform`)) false false)
    (set `self.Count` (+ (`self.Count`) 1) :!label _label_3)
    (elif (== _returnvalue 1)
      (`self.K2_SetActorTransform` (`self.otherPlaerRef`) (`|GetArrayItem` (`self.PlayerTransform`) 1) false false)
      (goto _label_3)
      (elif (== _returnvalue 2)
        (`self.K2_SetActorTransform` (`self.otherPlaerRef`) (`|GetArrayItem` (`self.PlayerTransform`) 2) false false)
        (goto _label_3)
        (elif (== _returnvalue 3)
          (`self.K2_SetActorTransform` (`self.otherPlaerRef`) (`|GetArrayItem` (`self.PlayerTransform`) 3) false false)
          (goto _label_3))))))

(fn `UserConstructionScript`)