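; Acceleration zone for a multi-ball lane that spins up balls while they are inside its trigger.
; Begin overlap matches balls against the spawn switch's ball array or the GameMode's main ball, then starts one of four timelines, letting several balls accelerate independently.
; Timeline curves scale a torque applied to each ball's physics along a selectable positive or negative X or Y axis.
; End overlap stops the matching timeline.
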(event `acceleBall1`
  (params (Ball :type "/Game/Workbench/BliePrint/2F/BP_BallPhysics Object Reference"))
  (`/Engine/EditorBlueprintResources/StandardMacros.IsValid` Ball
    (:`Is Valid`
      (bind (_direction _accelex) (`Timeline|accele` :!via `PlayFromStart` :!label _label)
        (:`Update`
          (`self.AddTorque` _accelex (`/Game/Workbench/BliePrint/2F/BP_BallPhysics.physics` Ball)))))))

(event `self.Trigger.OnComponentBeginOverlap`
  (params (OverlappedComponent :type "PrimitiveComponent Object Reference") (OtherActor :type "Actor Object Reference") (OtherComp :type "PrimitiveComponent Object Reference") (OtherBodyIndex :type Integer) (bFromSweep :type Boolean) (SweepResult :type "HitResult Structure (by ref)"))
  (bind _bp_ball (`/Game/Workbench/BP_Gamemode.BP_Ball` (cast `/Game/Workbench/BP_Gamemode` (`GameplayStatics.GetGameMode`) :!pure true)))
  (for (_array_element _array_index) (`/Game/Workbench/BliePrint/1F/Switch/BP_SpawnSwitch.BallPhysicsRefs` (`self.SapwnSwitchRef`))
    (if (== OtherActor _array_element)
      (if (== _array_index 0)
        (`self.acceleBall1` _array_element)
        (elif (== _array_index 1)
          (`self.acceleBall2` _array_element)
          (else
            (`self.acceleBall3` _array_element))))))
  (if (== OtherActor _bp_ball)
    (`self.acceleBall4` _bp_ball)))

(event `acceleBallStop1`
  (goto _label :!via `Stop`))

(event `acceleBall2`
  (params (Ball :type "/Game/Workbench/BliePrint/2F/BP_BallPhysics Object Reference"))
  (`/Engine/EditorBlueprintResources/StandardMacros.IsValid` Ball
    (:`Is Valid`
      (bind (_direction _accelex) (`Timeline|accele2` :!via `PlayFromStart` :!label _label_2)
        (:`Update`
          (`self.AddTorque` _accelex (`/Game/Workbench/BliePrint/2F/BP_BallPhysics.physics` Ball)))))))

(event `acceleBallStop2`
  (goto _label_2 :!via `Stop`))

(event `acceleBall3`
  (params (`ターゲット` :type "/Game/Workbench/BliePrint/2F/BP_BallPhysics Object Reference"))
  (`/Engine/EditorBlueprintResources/StandardMacros.IsValid` `ターゲット`
    (:`Is Valid`
      (bind (_direction _accelex) (`Timeline|accele3` :!via `PlayFromStart` :!label _label_3)
        (:`Update`
          (`self.AddTorque` _accelex (`/Game/Workbench/BliePrint/2F/BP_BallPhysics.physics` `ターゲット`)))))))

(event `self.Trigger.OnComponentEndOverlap`
  (params (OverlappedComponent :type "PrimitiveComponent Object Reference") (OtherActor :type "Actor Object Reference") (OtherComp :type "PrimitiveComponent Object Reference") (OtherBodyIndex :type Integer))
  (for (_array_element _array_index) (`/Game/Workbench/BliePrint/1F/Switch/BP_SpawnSwitch.BallPhysicsRefs` (`self.SapwnSwitchRef`))
    (if (== OtherActor _array_element)
      (if (== _array_index 0)
        (`self.acceleBallStop1`)
        (elif (== _array_index 1)
          (`self.acceleBallStop2`)
          (else
            (`self.acceleBallStop3`))))))
  (if (== OtherActor (`/Game/Workbench/BP_Gamemode.BP_Ball` (cast `/Game/Workbench/BP_Gamemode` (`GameplayStatics.GetGameMode`) :!pure true)))
    (`self.acceleBallStop4`)))

(event `acceleBallStop3`
  (goto _label_3 :!via `Stop`))

(event `acceleBall4`
  (params (`ターゲット` :type "/Game/Workbench/BliePrint/2F/BP_BallPhysics Object Reference"))
  (`/Engine/EditorBlueprintResources/StandardMacros.IsValid` `ターゲット`
    (:`Is Valid`
      (bind (_direction _accelex) (`Timeline|タイムライン_0` :!via `PlayFromStart` :!label _label_4)
        (:`Update`
          (`self.AddTorque` _accelex (`/Game/Workbench/BliePrint/2F/BP_BallPhysics.physics` `ターゲット`)))))))

(event `acceleBallStop4`
  (goto _label_4 :!via `Stop`))

(event `AddTorque`
  (params (Accele :type "Float (double-precision)") (Physics :type "PrimitiveComponent Object Reference"))
  (bind _torque (`self.Torque`))
  (`PrimitiveComponent.AddTorqueInRadians` Physics (select `int` (`self.Direction(-Y,Y,X,-X)`) :`0` (`KismetMathLibrary.MakeVector` (* Accele _torque)) :`1` (`KismetMathLibrary.MakeVector` (* Accele _torque -1.0)) :`2` (`KismetMathLibrary.MakeVector` 0.0 (* Accele _torque)) :`3` (`KismetMathLibrary.MakeVector` 0.0 (* Accele _torque -1.0))) "None" false))

(fn `UserConstructionScript`)