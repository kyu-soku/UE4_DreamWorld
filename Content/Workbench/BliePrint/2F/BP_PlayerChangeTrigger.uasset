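; BP_PlayerChangeTrigger swaps player control between two characters, SelfPlayer and OtherPlayerRef.
; ChangePlayer calls PlayerOnPlate, which swaps immediately if NonPlateChange is set, otherwise only when both characters' capsules overlap this trigger.
; CharacterChange disables movement on the currently possessed character, then after a short delay has the player controller possess the other one.
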(event `PlayerOnPlate?`
  (if (`self.NonPlateChange`)
    (`self.CharacterChange`)
    (else
      (set `self.Overlapping Actors(otherPlayer)` (`PrimitiveComponent.GetOverlappingActors` (`Character.CapsuleComponent` (`self.OtherPlayerRef`)) "/Script/Engine.Actor"))
      (for _array_element (`self.Overlapping Actors(otherPlayer)`)
        (if (== _array_element self)
          (set `self.Overlapping Actors(selfPlayer)` (`PrimitiveComponent.GetOverlappingActors` (`Character.CapsuleComponent` (`self.SelfPlayer`)) "/Script/Engine.Actor"))
          (for _array_element_2 (`self.Overlapping Actors(selfPlayer)`)
            (if (== _array_element_2 self)
              (`self.CharacterChange`))))))))

(event `/Game/Workbench/BliePrint/1F/BPI_Rkey.ChangePlayer`
  (`self.PlayerOnPlate?`))

(event `CharacterChange`
  (bind _returnvalue (`GameplayStatics.GetPlayerController` 0))
  (if (== (`self.SelfPlayer`) (`GameplayStatics.GetPlayerPawn` 0))
    (`CharacterMovementComponent.DisableMovement` (`Character.CharacterMovement` (`self.SelfPlayer`)))
    (`KismetSystemLibrary.Delay` 0.1)
    (`Controller.Possess` _returnvalue (`self.OtherPlayerRef`))
    (else
      (`CharacterMovementComponent.DisableMovement` (`Character.CharacterMovement` (`self.OtherPlayerRef`)))
      (`KismetSystemLibrary.Delay` 0.1)
      (`Controller.Possess` _returnvalue (`self.SelfPlayer`)))))

(fn `UserConstructionScript`)