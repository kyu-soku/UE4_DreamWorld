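; BP_SpawnSameMovement is a character that mirrors the player's jump and movement input.
; On BeginPlay it binds its jump, forward and right events to dispatchers on BP_PlayerController.
; Movement follows the player pawn's full control rotation, including pitch and roll, scaled by the controller's ForwardScale and RightScale.
; Jumping also prints a debug string.
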(event `self.ReceiveBeginPlay`
  (bind _asbp_player_controller (cast `/Game/Workbench/Player/BP_PlayerController` (`GameplayStatics.GetPlayerController` 0) :!pure true))
  (set `self.Player Controller` _asbp_player_controller)
  (add `/Game/Workbench/Player/BP_PlayerController.JumpEvent` _asbp_player_controller (delegate `JumpEvent`))
  (add `/Game/Workbench/Player/BP_PlayerController.MoveForward` (`self.Player Controller`) (delegate `MoveForward_イベント_0`))
  (add `/Game/Workbench/Player/BP_PlayerController.MoveRight` (`self.Player Controller`) (delegate `MoveRight_イベント_0`)))

(event `JumpEvent`
  (`self.Jump`)
  (`KismetSystemLibrary.PrintString` "jump"))

(event `MoveForward_イベント_0`
  (bind (_returnvalue_roll _returnvalue_pitch _returnvalue_yaw) (`KismetMathLibrary.BreakRotator` (`self.GetControlRotation` (`GameplayStatics.GetPlayerPawn` 0))))
  (`self.AddMovementInput` (`KismetMathLibrary.GetForwardVector` (`KismetMathLibrary.MakeRotator` _returnvalue_roll _returnvalue_pitch _returnvalue_yaw)) (`/Game/Workbench/Player/BP_PlayerController.ForwardScale` (`self.Player Controller`))))

(event `MoveRight_イベント_0`
  (bind (_returnvalue_roll _returnvalue_pitch _returnvalue_yaw) (`KismetMathLibrary.BreakRotator` (`self.GetControlRotation` (`GameplayStatics.GetPlayerPawn` 0))))
  (`self.AddMovementInput` (`KismetMathLibrary.GetRightVector` (`KismetMathLibrary.MakeRotator` _returnvalue_roll _returnvalue_pitch _returnvalue_yaw)) (`/Game/Workbench/Player/BP_PlayerController.RightScale` (`self.Player Controller`))))

(fn `UserConstructionScript`)