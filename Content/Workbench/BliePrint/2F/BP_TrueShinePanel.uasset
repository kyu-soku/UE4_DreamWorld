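; BP_TrueShinePanel is a panel Blueprint that takes on a gloss red, blue or green material when play begins.
; BeginPlay checks the boolean flags in DefaultColorSelect in red, blue, green priority and sets the matching material on element 1 of the Panel component.
; With no flag set the material stays unchanged, and the empty construction script means the choice is applied only at runtime.
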(event `self.ReceiveBeginPlay`
  (bind (_red _blue _green) (break `/Game/Workbench/BliePrint/2F/BPS_ColorFlag` (`self.DefaultColorSelect`)))
  (if _red
    (`PrimitiveComponent.SetMaterial` (`self.Panel`) 1 "/Game/Workbench/Material/M_GlossRed.M_GlossRed")
    (elif _blue
      (`PrimitiveComponent.SetMaterial` (`self.Panel`) 1 "/Game/Workbench/Material/M_GlossBlue.M_GlossBlue")
      (elif _green
        (`PrimitiveComponent.SetMaterial` (`self.Panel`) 1 "/Game/Workbench/Material/M_GlossGreen.M_GlossGreen")))))

(fn `UserConstructionScript`)