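; BP_ShinePanel is a color puzzle panel that cycles its material through red, blue and green each time its trigger is overlapped.
; BeginPlay applies the starting color from CurrentColorFlag, falling back to black when no color is set.
; Each color change updates the flag struct and compares it with TrueColorFlag.
; With a valid SpawnSwitchRef, a match sets ClearCondition and calls the switch's CheckCondition, while a mismatch clears it.
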(event `self.ReceiveBeginPlay`
  (`self.ChangeColor`))

(event `self.Trigger.OnComponentBeginOverlap`
  (params (OverlappedComponent :type "PrimitiveComponent Object Reference") (OtherActor :type "Actor Object Reference") (OtherComp :type "PrimitiveComponent Object Reference") (OtherBodyIndex :type Integer) (bFromSweep :type Boolean) (SweepResult :type "HitResult Structure (by ref)"))
  (bind _output_get (set `self.ColorChange` (+ (`self.ColorChange`) 1)))
  (bind _returnvalue (mod _output_get 3))
  (if (== _returnvalue 0)
    (`self.ChangeRed`)
    (elif (== _returnvalue 1)
      (`self.ChangeBlue`)
      (else
        (`self.ChangeGreen`)))))

(event `DefaultColor`
  (set `self.ColorChange` -1)
  (`PrimitiveComponent.SetMaterial` (`self.Panel`) 1 "/Game/Workbench/Material/M_Black.M_Black")
  (set `self.CurrentColorFlag` (make `/Game/Workbench/BliePrint/2F/BPS_ColorFlag` false))
  (`self.CheckColor`))

(event `ChangeRed`
  (`PrimitiveComponent.SetMaterial` (`self.Panel`) 1 "/Game/Workbench/Material/M_GlossRed.M_GlossRed")
  (set `self.CurrentColorFlag` (make `/Game/Workbench/BliePrint/2F/BPS_ColorFlag` true))
  (set `self.ColorChange` 0)
  (`self.CheckColor`))

(event `ChangeBlue`
  (`PrimitiveComponent.SetMaterial` (`self.Panel`) 1 "/Game/Workbench/Material/M_GlossBlue.M_GlossBlue")
  (set `self.CurrentColorFlag` (make `/Game/Workbench/BliePrint/2F/BPS_ColorFlag` false true))
  (set `self.ColorChange` 1)
  (`self.CheckColor`))

(event `ChangeGreen`
  (`PrimitiveComponent.SetMaterial` (`self.Panel`) 1 "/Game/Workbench/Material/M_GlossGreen.M_GlossGreen")
  (set `self.CurrentColorFlag` (make `/Game/Workbench/BliePrint/2F/BPS_ColorFlag` false false true))
  (set `self.ColorChange` 2)
  (`self.CheckColor`))

(event `ChangeColor`
  (bind (_red _blue _green) (break `/Game/Workbench/BliePrint/2F/BPS_ColorFlag` (`self.CurrentColorFlag`)))
  (if _red
    (`self.ChangeRed`)
    (elif _blue
      (`self.ChangeBlue`)
      (elif _green
        (`self.ChangeGreen`)
        (else
          (`self.DefaultColor`))))))

(event `CheckColor`
  (bind (_red _blue _green) (break `/Game/Workbench/BliePrint/2F/BPS_ColorFlag` (`self.CurrentColorFlag`)))
  (bind (_red_2 _blue_2 _green_2) (break `/Game/Workbench/BliePrint/2F/BPS_ColorFlag` (`self.TrueColorFlag`)))
  (`/Engine/EditorBlueprintResources/StandardMacros.IsValid` (`self.SpawnSwitchRef`)
    (:`Is Valid`
      (if (and (== _red _red_2) (== _blue _blue_2) (== _green _green_2))
        (set `self.ClearCondition` true)
        (`/Game/Workbench/BliePrint/1F/BP_SpawnSw.CheckCondition` (`self.SpawnSwitchRef`))
        (else
          (set `self.ClearCondition` false))))))

(fn `UserConstructionScript`)