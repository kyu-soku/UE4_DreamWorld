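; Warp point actor that teleports the player between linked warps through a selection menu.
; Interaction, gated by its own UsedWarps flag, opens WBP_WarpSelect and freezes movement until one of three buttons is clicked.
; An unlocked choice spawns a particle, waits, then moves the player to that warp.
; It also flags this warp in the destination's UsedWarps and, for a different destination, passes this warp to BP_GameInstance.
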(event `WarpEvent`
  (params (NewParam :type "Actor Object Reference"))
  (bind _charactermovement (`Character.CharacterMovement` (`self.CharacterRef`)))
  (`/Engine/EditorBlueprintResources/StandardMacros.DoOnce` false :!label _label
    (:`Completed`
      (`CharacterMovementComponent.DisableMovement` _charactermovement)
      (`GameplayStatics.SpawnEmitterAtLocation` "/Game/Workbench/Particle/P_Warp.P_Warp" (`SceneComponent.K2_GetComponentLocation` (`self.warp`)) (struct) (1.0 1.0 1.0) false)
      (`KismetSystemLibrary.Delay` 3.0)
      (`self.K2_SetActorTransform` (`GameplayStatics.GetPlayerPawn` 0) (`self.GetTransform` NewParam) false false)
      (`CharacterMovementComponent.SetMovementMode` _charactermovement "MOVE_Walking" 0)
      (goto _label :!via `Reset`))))

(event `/Game/Workbench/BliePrint/1F/BPI_Interact.HasInteracted`
  (if (`|GetArrayItem` (`self.UsedWarps`) (`KismetArrayLibrary.Array_Find` (`self.BP_Warp`) self))
    (`/Engine/EditorBlueprintResources/StandardMacros.DoOnce` false :!label _label_2
      (:`Completed`
        (`UserWidget.AddToViewport` (`self.WrapSelectRef`) 0)
        (set `PlayerController.bShowMouseCursor` true (`GameplayStatics.GetPlayerController` 0))
        (`CharacterMovementComponent.DisableMovement` (`Character.CharacterMovement` (`self.CharacterRef`)))
        (add `Button.OnClicked` (`/Game/Workbench/BliePrint/1F_sub/WBP_WarpSelect.1` (`self.WrapSelectRef`)) (delegate `OnClickedEvent`))
        (add `Button.OnClicked` (`/Game/Workbench/BliePrint/1F_sub/WBP_WarpSelect.3` (`self.WrapSelectRef`)) (delegate `OnClickedEvent`))
        (add `Button.OnClicked` (`/Game/Workbench/BliePrint/1F_sub/WBP_WarpSelect.2` (`self.WrapSelectRef`)) (delegate `OnClickedEvent`))))))

(event `self.ReceiveBeginPlay`
  (bind _returnvalue (`|CreateWidget` "/Game/Workbench/BliePrint/1F_sub/WBP_WarpSelect.WBP_WarpSelect_C"))
  (set `self.WrapSelectRef` _returnvalue)
  (set `self.CharacterRef` (cast `Character` (`GameplayStatics.GetPlayerPawn` 0) :!pure true)))

(event `OnClickedEvent`
  (bind _returnvalue (`KismetArrayLibrary.Array_Find` (`self.BP_Warp`) self))
  (bind _index (`/Game/Workbench/BliePrint/1F_sub/WBP_WarpSelect.Index` (`self.WrapSelectRef`)))
  (bind _output (`|GetArrayItem` (`self.BP_Warp`) _index))
  (`CharacterMovementComponent.SetMovementMode` (`Character.CharacterMovement` (`self.CharacterRef`)) "MOVE_Walking" 0)
  (`Widget.RemoveFromParent` (`self.WrapSelectRef`))
  (set `PlayerController.bShowMouseCursor` false (`GameplayStatics.GetPlayerController` 0))
  (if (`|GetArrayItem` (`self.UsedWarps`) _index)
    (`self.WarpEvent` _output)
    (`KismetArrayLibrary.Array_Set` (`/Game/Workbench/BliePrint/1F_sub/BP_Warp_test.UsedWarps` _output) _returnvalue true)
    (if (!= (`/Game/Workbench/BliePrint/1F_sub/WBP_WarpSelect.Index` (`self.WrapSelectRef`)) _returnvalue)
      (`/Game/Workbench/BP_GameInstance.Set Warp Map Test` (cast `/Game/Workbench/BP_GameInstance` (`GameplayStatics.GetGameInstance`) :!pure true) (`|GetArrayItem` (`self.BP_Warp`) _returnvalue))
      (goto _label_2 :!via `Reset`)
      (else
        (goto _label_2 :!via `Reset`)))
    (else
      (goto _label_2 :!via `Reset`))))

(fn `UserConstructionScript`)