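; A trigger volume that switches the player's view to an assigned camera actor with a timed blend, and blends back to the player on exit.
; Overlap events, optionally delayed, also toggle the game mode's camera-change flag.
; On entry it copies its forward and right axis and sign settings to the game instance as camera direction flags, which are not reset on exit.
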(event `self.Trigger.OnComponentBeginOverlap`
  (params (OverlappedComponent :type "PrimitiveComponent Object Reference") (OtherActor :type "Actor Object Reference") (OtherComp :type "PrimitiveComponent Object Reference") (OtherBodyIndex :type Integer) (bFromSweep :type Boolean) (SweepResult :type "HitResult Structure (by ref)"))
  (bind _asbp_game_instance (cast `/Game/Workbench/BP_GameInstance` (`GameplayStatics.GetGameInstance`) :!pure true))
  (if (`self.delay`)
    (`KismetSystemLibrary.Delay` 0.5))
  (bind _asbp_player (cast `/Game/Workbench/Player/BP_Player` OtherActor))
  (if (`KismetSystemLibrary.IsValid` _asbp_player)
    (bind _asplayer_controller (cast `PlayerController` (`Pawn.GetController` _asbp_player)))
    (if (`KismetSystemLibrary.IsValid` _asplayer_controller)
      (`PlayerController.SetViewTargetWithBlend` _asplayer_controller (`self.CameraActor`) (`self.CmeraBlendTime`) "VTBlend_Linear" 0.0 false)
      (set `/Game/Workbench/BP_Gamemode.CameraChenge` true (cast `/Game/Workbench/BP_Gamemode` (`GameplayStatics.GetGameMode`) :!pure true))
      (if (`self.ForwardDirectionWorldX`)
        (set `/Game/Workbench/BP_GameInstance.CameraForwardDirectionX` true _asbp_game_instance)
        (else
          (set `/Game/Workbench/BP_GameInstance.CameraForwardDirectionX` false _asbp_game_instance)))
      (if (`self.ForwardDirectionPositive`)
        (set `/Game/Workbench/BP_GameInstance.CameraForwardDirectionPositive` true _asbp_game_instance)
        (else
          (set `/Game/Workbench/BP_GameInstance.CameraForwardDirectionPositive` false _asbp_game_instance)))
      (if (`self.RightDirectionWorldX`)
        (set `/Game/Workbench/BP_GameInstance.CameraRightDirectionX` true _asbp_game_instance)
        (else
          (set `/Game/Workbench/BP_GameInstance.CameraRightDirectionX` false _asbp_game_instance)))
      (if (`self.RightDirectionWorldPositive`)
        (set `/Game/Workbench/BP_GameInstance.CameraRightDirectionPositive` true _asbp_game_instance)
        (else
          (set `/Game/Workbench/BP_GameInstance.CameraRightDirectionPositive` false _asbp_game_instance))))))

(event `self.Trigger.OnComponentEndOverlap`
  (params (OverlappedComponent :type "PrimitiveComponent Object Reference") (OtherActor :type "Actor Object Reference") (OtherComp :type "PrimitiveComponent Object Reference") (OtherBodyIndex :type Integer))
  (if (`self.delay`)
    (`KismetSystemLibrary.Delay` 0.5))
  (bind _asbp_player (cast `/Game/Workbench/Player/BP_Player` OtherActor))
  (if (`KismetSystemLibrary.IsValid` _asbp_player)
    (bind _asplayer_controller (cast `PlayerController` (`Pawn.GetController` _asbp_player)))
    (if (`KismetSystemLibrary.IsValid` _asplayer_controller)
      (`PlayerController.SetViewTargetWithBlend` _asplayer_controller _asbp_player (`self.CmeraBlendTime`) "VTBlend_Linear" 0.0 false)
      (set `/Game/Workbench/BP_Gamemode.CameraChenge` false (cast `/Game/Workbench/BP_Gamemode` (`GameplayStatics.GetGameMode`) :!pure true)))))

(fn `UserConstructionScript`)