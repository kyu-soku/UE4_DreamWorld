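; BP_ConstantMovePlate is a moving plate that travels along selected local axes, driven by a timeline.
; On BeginPlay, the UpDown timeline plays at a rate of 1/RoundTripTime, interpolating an offset between zero and Distance.
; Every Tick applies that offset as the Plate's relative location on each axis enabled in Direction, zeroing the other axes.
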(event `self.ReceiveBeginPlay`
  ;[1 1 1] 上下移動
  (`TimelineComponent.SetPlayRate` (`self.UpDown`) (/ 1.0 (`self.RoundTripTime`)))
  (bind (_direction `_新規track_0`) (`Timeline|UpDown`)
    (:`Update`
      (bind _output_get (set `self.Location` (`KismetMathLibrary.Lerp` 0.0 (`self.Distance`) `_新規track_0`))))))

(event `self.ReceiveTick`
  (params (DeltaSeconds :type "Float (single-precision)"))
  (bind _location (`self.Location`))
  (bind (_directionx _directiony _directionz) (break `/Game/Workbench/BliePrint/1F/BPS_Direction` (`self.Direction`)))
  ;[1 1 1] 上下移動
  (if _directionx
    (set `self.LocationX` _location)
    (else
      (set `self.LocationX` 0.0)))
  (if _directiony
    (set `self.LocationY` _location)
    (else
      (set `self.LocationY` 0.0)))
  (if _directionz
    (bind _output_get (set `self.LocationZ` _location))
    (else
      (set `self.LocationZ` 0.0)))
  (`SceneComponent.K2_SetRelativeLocation` (`self.Plate`) (`KismetMathLibrary.MakeVector` (`self.LocationX`) (`self.LocationY`) (`self.LocationZ`)) false false))

(fn `UserConstructionScript`)