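; BP_Warp is a warp point that moves the player pawn to a destination actor's transform.
; At BeginPlay it creates a signboard widget, which the Trigger overlap shows and hides only if the game instance's UsedWarpSample flag was set at that time.
; HasInteracted calls CallWarpPareGet, while WarpEvent receives the destination, removes the signboard, disables movement and spawns a particle effect.
; After a short delay, WarpEvent relocates the player and restores walking.
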(event `self.ReceiveBeginPlay`
  (bind _returnvalue (`|CreateWidget` "/Game/Workbench/BliePrint/1F/WBP_Signboard.WBP_Signboard_C"))
  (set `self.SignboardRef` _returnvalue)
  (bind _asbp_game_instance (cast `/Game/Workbench/BP_GameInstance` (`GameplayStatics.GetGameInstance`)))
  (if (`/Game/Workbench/BP_GameInstance.UsedWarp_sample` _asbp_game_instance)
    (set `self.display` true)))

(event `self.Trigger.OnComponentBeginOverlap`
  (params (OverlappedComponent :type "PrimitiveComponent Object Reference") (OtherActor :type "Actor Object Reference") (OtherComp :type "PrimitiveComponent Object Reference") (OtherBodyIndex :type Integer) (bFromSweep :type Boolean) (SweepResult :type "HitResult Structure (by ref)"))
  (if (and (== OtherActor (`GameplayStatics.GetPlayerPawn` 0)) (`self.display`))
    (`UserWidget.AddToViewport` (`self.SignboardRef`) 0)))

(event `self.Trigger.OnComponentEndOverlap`
  (params (OverlappedComponent :type "PrimitiveComponent Object Reference") (OtherActor :type "Actor Object Reference") (OtherComp :type "PrimitiveComponent Object Reference") (OtherBodyIndex :type Integer))
  (if (and (`self.display`) (== (`GameplayStatics.GetPlayerPawn` 0) OtherActor))
    (`Widget.RemoveFromParent` (`self.SignboardRef`))))

(event `/Game/Workbench/BliePrint/1F/BPI_Interact.HasInteracted`
  (`self.WarpPareGet`))

(event `WarpEvent`
  (params (NewParam :type "Actor Object Reference"))
  (bind _charactermovement (`Character.CharacterMovement` (cast `Character` (`GameplayStatics.GetPlayerPawn` 0) :!pure true)))
  (`Widget.RemoveFromParent` (`self.SignboardRef`))
  (`CharacterMovementComponent.DisableMovement` _charactermovement)
  (`GameplayStatics.SpawnEmitterAtLocation` "/Game/Workbench/Particle/P_Warp.P_Warp" (`SceneComponent.K2_GetComponentLocation` (`self.warp`)) (struct) (1.0 1.0 1.0) false)
  (`KismetSystemLibrary.Delay` 3.0)
  (`self.K2_SetActorTransform` (`GameplayStatics.GetPlayerPawn` 0) (`self.GetTransform` NewParam) false false)
  (`CharacterMovementComponent.SetMovementMode` _charactermovement "MOVE_Walking" 0))

(fn `UserConstructionScript`)