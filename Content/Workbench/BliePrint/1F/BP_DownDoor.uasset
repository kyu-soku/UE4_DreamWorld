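; BP_DownDoor is a door actor that lowers itself the first time the player enters its trigger.
; The trigger's overlap event checks for the player pawn and passes through a DoOnce, which is never reset, to the DownDoor event.
; DownDoor plays the Down timeline at a rate derived from MoveTime, using its curve to interpolate the Door's relative height from raised to lowered.
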(event `self.Trigger.OnComponentBeginOverlap`
  (params (OverlappedComponent :type "PrimitiveComponent Object Reference") (OtherActor :type "Actor Object Reference") (OtherComp :type "PrimitiveComponent Object Reference") (OtherBodyIndex :type Integer) (bFromSweep :type Boolean) (SweepResult :type "HitResult Structure (by ref)"))
  (if (== OtherActor (`GameplayStatics.GetPlayerPawn` 0))
    (`/Engine/EditorBlueprintResources/StandardMacros.DoOnce` false
      (:`Completed`
        (`self.DownDoor`)))))

(event `DownDoor`
  (`TimelineComponent.SetPlayRate` (`self.Down`) (/ 1.0 (`self.MoveTime`)))
  (bind (_direction _downz) (`Timeline|Down`)
    (:`Update`
      (`SceneComponent.K2_SetRelativeLocation` (`self.Door`) (`KismetMathLibrary.MakeVector` 0.0 0.0 (`KismetMathLibrary.Lerp` 550.0 150.0 _downz)) false false))))

(fn `UserConstructionScript`)