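; Readable signboard actor that shows different text depending on whether the player reads it from the front, back or top.
; Front, Back and UP overlap volumes set the side flags and show a WBP_Signboard widget created at BeginPlay, resetting and removing it on exit.
; HasInteracted toggles between the press-E prompt and that side's text, turning the player's yaw toward the sign for front and back reads.
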(event `self.ReceiveBeginPlay`
  (bind _returnvalue (`|CreateWidget` "/Game/Workbench/BliePrint/1F/WBP_Signboard.WBP_Signboard_C"))
  (set `self.WBP_SignboardRef` _returnvalue))

(event `self.UP.OnComponentBeginOverlap`
  (params (OverlappedComponent :type "PrimitiveComponent Object Reference") (OtherActor :type "Actor Object Reference") (OtherComp :type "PrimitiveComponent Object Reference") (OtherBodyIndex :type Integer) (bFromSweep :type Boolean) (SweepResult :type "HitResult Structure (by ref)"))
  (if (== OtherActor (`GameplayStatics.GetPlayerPawn` 0))
    (`UserWidget.AddToViewport` (`self.WBP_SignboardRef`) 0)
    (set `self.CanView` false)
    (set `self.UpViewContents` true)))

(event `self.Front.OnComponentBeginOverlap`
  (params (OverlappedComponent :type "PrimitiveComponent Object Reference") (OtherActor :type "Actor Object Reference") (OtherComp :type "PrimitiveComponent Object Reference") (OtherBodyIndex :type Integer) (bFromSweep :type Boolean) (SweepResult :type "HitResult Structure (by ref)"))
  ;[1 1 1] オーバーラップで画面に表示(Front)
  (if (== OtherActor (`GameplayStatics.GetPlayerPawn` 0))
    (`UserWidget.AddToViewport` (`self.WBP_SignboardRef`) 0)
    (set `self.CanView` true)
    (set `self.UpViewContents` false)))

(event `self.Front.OnComponentEndOverlap`
  (params (OverlappedComponent :type "PrimitiveComponent Object Reference") (OtherActor :type "Actor Object Reference") (OtherComp :type "PrimitiveComponent Object Reference") (OtherBodyIndex :type Integer))
  (bind _wbp_signboardref (`self.WBP_SignboardRef`))
  ;[1 1 1] オーバーラップで画面に表示(Front)
  (if (== OtherActor (`GameplayStatics.GetPlayerPawn` 0))
    (`/Game/Workbench/BliePrint/1F/WBP_Signboard.SetPressEKey` _wbp_signboardref)
    (set `self.IsTextContents` false)
    (`Widget.RemoveFromParent` _wbp_signboardref)))

(event `self.UP.OnComponentEndOverlap`
  (params (OverlappedComponent :type "PrimitiveComponent Object Reference") (OtherActor :type "Actor Object Reference") (OtherComp :type "PrimitiveComponent Object Reference") (OtherBodyIndex :type Integer))
  (bind _wbp_signboardref (`self.WBP_SignboardRef`))
  (if (== OtherActor (`GameplayStatics.GetPlayerPawn` 0))
    (`/Game/Workbench/BliePrint/1F/WBP_Signboard.SetPressEKey` _wbp_signboardref)
    (set `self.IsTextContents` false)
    (`Widget.RemoveFromParent` _wbp_signboardref)))

(event `self.Back.OnComponentBeginOverlap`
  (params (OverlappedComponent :type "PrimitiveComponent Object Reference") (OtherActor :type "Actor Object Reference") (OtherComp :type "PrimitiveComponent Object Reference") (OtherBodyIndex :type Integer) (bFromSweep :type Boolean) (SweepResult :type "HitResult Structure (by ref)"))
  (if (== OtherActor (`GameplayStatics.GetPlayerPawn` 0))
    (`UserWidget.AddToViewport` (`self.WBP_SignboardRef`) 0)
    (set `self.CanView` false)
    (set `self.UpViewContents` false)))

(event `self.Back.OnComponentEndOverlap`
  (params (OverlappedComponent :type "PrimitiveComponent Object Reference") (OtherActor :type "Actor Object Reference") (OtherComp :type "PrimitiveComponent Object Reference") (OtherBodyIndex :type Integer))
  (bind _wbp_signboardref (`self.WBP_SignboardRef`))
  (if (== OtherActor (`GameplayStatics.GetPlayerPawn` 0))
    (`/Game/Workbench/BliePrint/1F/WBP_Signboard.SetPressEKey` _wbp_signboardref)
    (set `self.IsTextContents` false)
    (`Widget.RemoveFromParent` _wbp_signboardref)))

(event `/Game/Workbench/BliePrint/1F/BPI_Interact.HasInteracted`
  (bind _returnvalue (`GameplayStatics.GetPlayerPawn` 0))
  (bind _wbp_signboardref (`self.WBP_SignboardRef`))
  (bind (_returnvalue_roll _returnvalue_pitch _returnvalue_yaw) (`KismetMathLibrary.BreakRotator` (`KismetMathLibrary.FindLookAtRotation` (`self.K2_GetActorLocation` _returnvalue) (`self.K2_GetActorLocation`))))
  (if (`self.IsTextContents`)
    (`/Game/Workbench/BliePrint/1F/WBP_Signboard.SetPressEKey` _wbp_signboardref)
    (set `self.IsTextContents` false)
    (else
      (if (`self.UpViewContents`)
        ;[1 1 1] 看板の上から読もうとしたやつ
        (`/Game/Workbench/BliePrint/1F/WBP_Signboard.SetTextContents` _wbp_signboardref (`self.UpTextContens`))
        (else
          ;[1 1 1] 看板に注目する
          (`self.K2_SetActorRelativeRotation` _returnvalue (`KismetMathLibrary.MakeRotator` 0.0 0.0 _returnvalue_yaw) false false)
          ;[1 1 1] 看板の後ろから読んでいるか前から読んでいるか
          (`/Game/Workbench/BliePrint/1F/WBP_Signboard.SetTextContents` _wbp_signboardref (select `bool` (`self.CanView`) :`false` (`self.CanNotView`) :`true` (`self.Contents`)))))
      (set `self.IsTextContents` true))))

(fn `UserConstructionScript`)