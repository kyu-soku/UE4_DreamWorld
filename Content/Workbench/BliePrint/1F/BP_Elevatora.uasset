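; Interactable elevator actor that moves its Elevator component along X, Y, then Z, and retraces Z, Y, X on the next interaction.
; A DoOnce blocks retriggering until the Delay-sequenced legs end, while FlipFlops alternate direction.
; Each axis lerps relative location on its own timeline, but all three set play rate only on the X timeline (DirectionMove).
; An unconnected single-timeline diagonal move remains unused.
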(event `/Game/Workbench/BliePrint/1F/BPI_Interact.HasInteracted`
  (`self.MoveElevator`))

(event `MoveElevator`
  (bind _movetimez (`self.MoveTimeZ`))
  (bind _movetimex (`self.MoveTimeX`))
  (bind _movetimex_2 (`self.MoveTimeX`))
  (bind _movetimey (`self.MoveTimeY`))
  (bind _movetimey_2 (`self.MoveTimeY`))
  (bind _movetimez_2 (`self.MoveTimeZ`))
  (`/Engine/EditorBlueprintResources/StandardMacros.DoOnce` false :!label _label
    (:`Completed`
      (`/Engine/EditorBlueprintResources/StandardMacros.FlipFlop`
        (:`A`
          (`self.MoveDirectionX` (`self.DistanceX`) _movetimex_2)
          (`KismetSystemLibrary.Delay` _movetimex_2)
          (`self.MoveDirectionY` (`self.DistanceY`) _movetimey_2)
          (`KismetSystemLibrary.Delay` _movetimey_2)
          (`self.MoveDirectionZ` (`self.DistanceZ`) _movetimez_2)
          (`KismetSystemLibrary.Delay` _movetimez_2)
          (goto _label :!via `Reset`))
        (:`B`
          (`self.MoveDirectionZ` (`self.DistanceZ`) _movetimez)
          (`KismetSystemLibrary.Delay` _movetimez)
          (`self.MoveDirectionY` (`self.DistanceY`) _movetimey)
          (`KismetSystemLibrary.Delay` _movetimey)
          (`self.MoveDirectionX` (`self.DistanceX`) _movetimex)
          (`KismetSystemLibrary.Delay` _movetimex)
          (goto _label :!via `Reset`))))))

(event `MoveDirectionX`
  (params (DirectionX :type "Float (double-precision)") (MoveTime :type "Float (double-precision)"))
  (bind _returnvalue (/ 1.0 MoveTime))
  (bind _directionmove (`self.DirectionMove`))
  (`/Engine/EditorBlueprintResources/StandardMacros.FlipFlop`
    (:`A`
      (`TimelineComponent.SetPlayRate` _directionmove _returnvalue)
      (bind (_direction _move) (`Timeline|DirectionMove` :!label _label_2)
        (:`Update`
          (`SceneComponent.K2_SetRelativeLocation` (`self.Elevator`) (`KismetMathLibrary.MakeVector` (`KismetMathLibrary.Lerp` 0.0 DirectionX _move)) false false))))
    (:`B`
      (`TimelineComponent.SetPlayRate` _directionmove _returnvalue)
      (goto _label_2 :!via `Reverse`))))

(event `MoveDirectionY`
  (params (DirectionY :type "Float (double-precision)") (MoveTime :type "Float (double-precision)"))
  (bind _returnvalue (/ 1.0 MoveTime))
  (bind _directionmove (`self.DirectionMove`))
  (`/Engine/EditorBlueprintResources/StandardMacros.FlipFlop`
    (:`A`
      (`TimelineComponent.SetPlayRate` _directionmove _returnvalue)
      (bind (_direction _move) (`Timeline|タイムライン_0` :!label _label_3)
        (:`Update`
          (`SceneComponent.K2_SetRelativeLocation` (`self.Elevator`) (`KismetMathLibrary.MakeVector` (`self.DistanceX`) (`KismetMathLibrary.Lerp` 0.0 DirectionY _move)) false false))))
    (:`B`
      (`TimelineComponent.SetPlayRate` _directionmove _returnvalue)
      (goto _label_3 :!via `Reverse`))))

(event `MoveDirectionZ`
  (params (DirectionZ :type "Float (double-precision)") (MoveTime :type "Float (double-precision)"))
  (bind _returnvalue (/ 1.0 MoveTime))
  (bind _directionmove (`self.DirectionMove`))
  (`/Engine/EditorBlueprintResources/StandardMacros.FlipFlop`
    (:`A`
      (`TimelineComponent.SetPlayRate` _directionmove _returnvalue)
      (bind (_direction _move) (`Timeline|タイムライン_1` :!label _label_4)
        (:`Update`
          (`SceneComponent.K2_SetRelativeLocation` (`self.Elevator`) (`KismetMathLibrary.MakeVector` (`self.DistanceX`) (`self.DistanceY`) (`KismetMathLibrary.Lerp` 0.0 DirectionZ _move)) false false))))
    (:`B`
      (`TimelineComponent.SetPlayRate` _directionmove _returnvalue)
      (goto _label_4 :!via `Reverse`))))

(fn `UserConstructionScript`)