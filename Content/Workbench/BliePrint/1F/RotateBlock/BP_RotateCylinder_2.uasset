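; Rotating cylinder block that slides along its local Y axis when the player enters its trigger.
; A Rotate timeline starts at BeginPlay and rolls the cylinder, paced by RotateTime.
; After a one-second delay, overlap plays a Move timeline that carries cylinder and trigger toward Distance over MoveTime.
; Leaving the trigger stops the movement in place but does not cancel a pending delay.
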(event `self.ReceiveBeginPlay`
  (`TimelineComponent.SetPlayRate` (`self.Rotate`) (/ 1.0 (`self.RotateTime`)))
  (bind (_direction _rotate) (`Timeline|Rotate`)
    (:`Update`
      (`SceneComponent.K2_SetRelativeRotation` (`self.Cylinder`) (`KismetMathLibrary.MakeRotator` (`KismetMathLibrary.Lerp` 0.0 -359.0 _rotate) -90.0) false false))))

(event `self.Trigger.OnComponentBeginOverlap`
  (params (OverlappedComponent :type "PrimitiveComponent Object Reference") (OtherActor :type "Actor Object Reference") (OtherComp :type "PrimitiveComponent Object Reference") (OtherBodyIndex :type Integer) (bFromSweep :type Boolean) (SweepResult :type "HitResult Structure (by ref)"))
  (if (== OtherActor (`GameplayStatics.GetPlayerPawn` 0))
    (`KismetSystemLibrary.Delay` 1.0)
    (`TimelineComponent.SetPlayRate` (`self.Move`) (/ 1.0 (`self.MoveTime`)))
    (bind (_direction _move) (`Timeline|Move` :!label _label)
      (:`Update`
        (bind _returnvalue (`KismetMathLibrary.Lerp` 0.0 (`self.Distance`) _move))
        (`SceneComponent.K2_SetRelativeLocation` (`self.Cylinder`) (`KismetMathLibrary.MakeVector` 0.0 _returnvalue) false false)
        (`SceneComponent.K2_SetRelativeLocation` (`self.Trigger`) (`KismetMathLibrary.MakeVector` 0.0 _returnvalue 300.0) false false))
      (:`Finished`
        (`KismetSystemLibrary.PrintString` "完了")))))

(event `self.Trigger.OnComponentEndOverlap`
  (params (OverlappedComponent :type "PrimitiveComponent Object Reference") (OtherActor :type "Actor Object Reference") (OtherComp :type "PrimitiveComponent Object Reference") (OtherBodyIndex :type Integer))
  (if (== OtherActor (`GameplayStatics.GetPlayerPawn` 0))
    (`KismetSystemLibrary.PrintString` "Stop")
    (goto _label :!via `Stop`)))

(fn `UserConstructionScript`)