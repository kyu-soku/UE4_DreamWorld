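; Blue sphere item actor with four animated rings that disappears when the player touches it.
; Shortly after BeginPlay it destroys itself if the GameInstance's blue jewel flag is set, otherwise it plays a Rotate timeline scaled by RotateTime.
; The timeline spins each ring on its own orientation, and GetTrigger overlap with the player pawn destroys the actor without setting the jewel flag here.
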(event `self.ReceiveBeginPlay`
  (`KismetSystemLibrary.Delay` 0.2)
  (if (`.BuleJewel` (`/Game/Workbench/BP_GameInstance.GetJewels` (cast `/Game/Workbench/BP_GameInstance` (`GameplayStatics.GetGameInstance`) :!pure true)))
    (`self.K2_DestroyActor`)
    (else
      (`TimelineComponent.SetPlayRate` (`self.Rotate`) (/ 1.0 (`self.RotateTime`)))
      (bind (_direction _rotate) (`Timeline|Rotate`)
        (:`Update`
          (bind _returnvalue (`KismetMathLibrary.Lerp` 0.0 -359.0 _rotate))
          (`SceneComponent.K2_SetRelativeRotation` (`self.ring1`) (`KismetMathLibrary.MakeRotator` _returnvalue) false false)
          (`SceneComponent.K2_SetRelativeRotation` (`self.ring2`) (`KismetMathLibrary.MakeRotator` 0.0 _returnvalue 0.0) false false)
          (`SceneComponent.K2_SetRelativeRotation` (`self.ring3`) (`KismetMathLibrary.MakeRotator` _returnvalue 90.0) false false)
          (`SceneComponent.K2_SetRelativeRotation` (`self.ring4`) (`KismetMathLibrary.MakeRotator` 0.0 _returnvalue 90.0) false false))))))

(event `self.GetTrigger.OnComponentBeginOverlap`
  (params (OverlappedComponent :type "PrimitiveComponent Object Reference") (OtherActor :type "Actor Object Reference") (OtherComp :type "PrimitiveComponent Object Reference") (OtherBodyIndex :type Integer) (bFromSweep :type Boolean) (SweepResult :type "HitResult Structure (by ref)"))
  (if (== OtherActor (`GameplayStatics.GetPlayerPawn` 0))
    (`self.K2_DestroyActor`)))

(fn `UserConstructionScript`)