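; BP_Warp_NonExplain is an interactable warp point that moves the player to the first linked warp in BPWarp.
; When UsedWarp is set, interaction disables movement, spawns P_Warp effects at both ends, then after a delay applies the destination's transform and restores walking.
; A resettable DoOnce blocks re-entry during the warp.
; The first interaction also enables the destination's UsedWarp and saves it through BP_GameInstance.
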(event `WarpEvent`
  (params (NewParam :type "Actor Object Reference"))
  (bind _charactermovement (`Character.CharacterMovement` (cast `Character` (`GameplayStatics.GetPlayerPawn` 0) :!pure true)))
  (`/Engine/EditorBlueprintResources/StandardMacros.DoOnce` false :!label _label
    (:`Completed`
      (`CharacterMovementComponent.DisableMovement` _charactermovement)
      (`GameplayStatics.SpawnEmitterAtLocation` "/Game/Workbench/Particle/P_Warp.P_Warp" (`SceneComponent.K2_GetComponentLocation` (`self.warp`)) (struct) (1.0 1.0 1.0) false)
      (`GameplayStatics.SpawnEmitterAtLocation` "/Game/Workbench/Particle/P_Warp.P_Warp" (`SceneComponent.K2_GetComponentLocation` (`/Game/Workbench/BliePrint/1F/BP_Warp_NonExplain.warp` (`|GetArrayItem` (`self.BP_Warp`)))) (struct) (1.0 1.0 1.0) false)
      (`KismetSystemLibrary.Delay` 1.0)
      (`self.K2_SetActorTransform` (`GameplayStatics.GetPlayerPawn` 0) (`self.GetTransform` NewParam) false false)
      (`CharacterMovementComponent.SetMovementMode` _charactermovement "MOVE_Walking" 0)
      (goto _label :!via `Reset`))))

(event `/Game/Workbench/BliePrint/1F/BPI_Interact.HasInteracted`
  (bind _output (`|GetArrayItem` (`self.BP_Warp`)))
  (if (`self.UsedWarp`)
    (`self.WarpEvent` _output)
    (`/Engine/EditorBlueprintResources/StandardMacros.DoOnce` false
      (:`Completed`
        (set `/Game/Workbench/BliePrint/1F/BP_Warp_NonExplain.UsedWarp` true _output)
        (`/Game/Workbench/BP_GameInstance.SetSaveUsedWarp` (cast `/Game/Workbench/BP_GameInstance` (`GameplayStatics.GetGameInstance`) :!pure true) _output)))))

(fn `UserConstructionScript`)