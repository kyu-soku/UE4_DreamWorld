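; BP_SpawnSw is a pressure switch that respawns physics balls and resets its linked puzzle panels.
; Overlapping the trigger runs a timeline that lowers the switch; when fully pressed, it replaces one ball (registered with the GameMode) or several from a transform array.
; Each spawn restores ShinePanel colors cached at BeginPlay.
; A separate CheckCondition function opens the linked door once all panels are clear, saving it in the GameInstance.
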(event `self.ReceiveBeginPlay`
  (bind _shinepanel (`self.ShinePanel`))
  (for _array_element _shinepanel
    (`KismetArrayLibrary.Array_Add` (`self.DefaultColor`) (`/Game/Workbench/BliePrint/2F/BP_ShinePanel.CurrentColorFlag` _array_element)))
  (set `self.ShinePanelLength` (`KismetArrayLibrary.Array_Length` _shinepanel)))

(event `self.Trigger.OnComponentBeginOverlap`
  (params (OverlappedComponent :type "PrimitiveComponent Object Reference") (OtherActor :type "Actor Object Reference") (OtherComp :type "PrimitiveComponent Object Reference") (OtherBodyIndex :type Integer) (bFromSweep :type Boolean) (SweepResult :type "HitResult Structure (by ref)"))
  (bind (_direction _onoff) (`Timeline|ONOFF` :!label _label)
    (:`Update`
      (`SceneComponent.K2_SetRelativeLocation` (`self.Switch`) (`KismetMathLibrary.VLerp` (0.0 0.0 12.1) (0.0 0.0 0.1) _onoff) false false))
    (:`Finished`
      (if (== _onoff 1.0)
        (if (`self.ManySpawn`)
          (`self.ManySpawn(Max3)`)
          (else
            (`self.Spawn`)))))))

(event `self.Trigger.OnComponentEndOverlap`
  (params (OverlappedComponent :type "PrimitiveComponent Object Reference") (OtherActor :type "Actor Object Reference") (OtherComp :type "PrimitiveComponent Object Reference") (OtherBodyIndex :type Integer))
  (goto _label :!via `Reverse`))

(event `Spawn`
  (bind _ballphysicsref (`self.BallPhysicsRef`))
  (`/Engine/EditorBlueprintResources/StandardMacros.IsValid` _ballphysicsref
    (:`Is Valid`
      (`self.K2_DestroyActor` _ballphysicsref))
    (:`Is Not Valid`
      _))
  (bind _returnvalue (`|SpawnActorFromClass` "/Game/Workbench/BliePrint/2F/BP_BallPhysics.BP_BallPhysics_C" (`self.SpawnTransform`) "Undefined" "OverrideRootScale" null null))
  (bind _output_get (set `self.BallPhysicsRef` _returnvalue))
  (set `/Game/Workbench/BP_Gamemode.BP_Ball` _output_get (cast `/Game/Workbench/BP_Gamemode` (`GameplayStatics.GetGameMode`) :!pure true))
  (`self.ResetColor`))

(event `ResetColor`
  (for (_array_element _array_index) (`self.ShinePanel`)
    (set `/Game/Workbench/BliePrint/2F/BP_ShinePanel.CurrentColorFlag` (`|GetArrayItem` (`self.DefaultColor`) _array_index) _array_element)
    (`/Game/Workbench/BliePrint/2F/BP_ShinePanel.ChangeColor` _array_element)))

(event `ManySpawn(Max3)`
  (for _array_element (`self.BallPhysicsRefs`)
    (`/Engine/EditorBlueprintResources/StandardMacros.IsValid` _array_element
      (:`Is Valid`
        (`self.K2_DestroyActor` _array_element))))
  (for (_array_element_2 _array_index) (`self.SpawnTransforms`)
    (bind _returnvalue (`|SpawnActorFromClass` "/Game/Workbench/BliePrint/2F/BP_BallPhysics.BP_BallPhysics_C" _array_element_2 "Undefined" "OverrideRootScale" null null))
    (`KismetArrayLibrary.Array_Set` (`self.BallPhysicsRefs`) _array_index _returnvalue))
  (`self.ResetColor`))

(fn `CheckCondition`
  (bind _paneldoorref (`self.PanelDoorRef`))
  (for _array_element (`self.ShinePanel`)
    (if (not (`/Game/Workbench/BliePrint/2F/BP_ShinePanel.ClearCondition` _array_element))
      (return)))
  (if (`/Game/Workbench/BliePrint/2F/BP_PanelDoor.alreadyOpen` _paneldoorref)
    (return)
    (else
      (`/Engine/EditorBlueprintResources/StandardMacros.DoOnce` false
        (:`Completed`
          (`/Game/Workbench/BliePrint/2F/BP_PanelDoor.Open` _paneldoorref)
          (`/Game/Workbench/BP_GameInstance.SetSavePanelDoor` (cast `/Game/Workbench/BP_GameInstance` (`GameplayStatics.GetGameInstance`) :!pure true) (`self.PanelDoorRef`))
          (return))))))

(fn `UserConstructionScript`)