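; BP_ElevatorEarliesta is an interactable elevator actor that travels between its start position and a configurable offset.
; HasInteracted calls MoveElevator, where a FlipFlop alternately plays and reverses the Move timeline at a rate derived from MoveTime.
; The timeline lerps the Elevator component's relative location from zero to DistanceX/Y/Z.
; A DoOnce gate ignores further triggers until the timeline finishes.
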(event `/Game/Workbench/BliePrint/1F/BPI_Interact.HasInteracted`
  (`self.MoveElevator`))

(event `MoveElevator`
  (bind _move (`self.move`))
  (bind _returnvalue (/ 1.0 (`self.MoveTime`)))
  (`/Engine/EditorBlueprintResources/StandardMacros.DoOnce` false :!label _label
    (:`Completed`
      (`/Engine/EditorBlueprintResources/StandardMacros.FlipFlop`
        (:`A`
          (`TimelineComponent.SetPlayRate` _move _returnvalue)
          (bind (_direction _move_2) (`Timeline|move` :!label _label_2)
            (:`Update`
              (`SceneComponent.K2_SetRelativeLocation` (`self.Elevator`) (`KismetMathLibrary.MakeVector` (`KismetMathLibrary.Lerp` 0.0 (`self.DistanceX`) _move_2) (`KismetMathLibrary.Lerp` 0.0 (`self.DistanceY`) _move_2) (`KismetMathLibrary.Lerp` 0.0 (`self.DistanceZ`) _move_2)) false false))
            (:`Finished`
              (goto _label :!via `Reset`))))
        (:`B`
          (`TimelineComponent.SetPlayRate` _move _returnvalue)
          (goto _label_2 :!via `Reverse`))))))

(fn `UserConstructionScript`)