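; BP_ElevatorSw is a pressure switch that calls an elevator once it is fully pressed.
; Overlapping the Trigger plays the ONOFF timeline to lower the Switch mesh, and leaving reverses it.
; When the timeline finishes fully on, ChangeElevator calls MoveElevator on either ElevatorEarliest or Elevator, chosen by the Earliest flag.
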(event `self.Trigger.OnComponentBeginOverlap`
  (params (OverlappedComponent :type "PrimitiveComponent Object Reference") (OtherActor :type "Actor Object Reference") (OtherComp :type "PrimitiveComponent Object Reference") (OtherBodyIndex :type Integer) (bFromSweep :type Boolean) (SweepResult :type "HitResult Structure (by ref)"))
  (bind (_direction _onoff) (`Timeline|ONOFF` :!label _label)
    (:`Update`
      (`SceneComponent.K2_SetRelativeLocation` (`self.Switch`) (`KismetMathLibrary.VLerp` (0.0 0.0 0.0) (0.0 0.0 -15.0) _onoff) false false))
    (:`Finished`
      (if (== _onoff 1.0)
        (`self.ChangeElevator`)))))

(event `self.Trigger.OnComponentEndOverlap`
  (params (OverlappedComponent :type "PrimitiveComponent Object Reference") (OtherActor :type "Actor Object Reference") (OtherComp :type "PrimitiveComponent Object Reference") (OtherBodyIndex :type Integer))
  (goto _label :!via `Reverse`))

(event `ChangeElevator`
  (if (`self.Earliest`)
    (`/Game/Workbench/BliePrint/1F/BP_ElevatorEarliesta.MoveElevator` (`self.ElevatorEarliest`))
    (else
      (`/Game/Workbench/BliePrint/1F/BP_Elevatora.MoveElevator` (`self.Elevator`)))))

(fn `UserConstructionScript`)