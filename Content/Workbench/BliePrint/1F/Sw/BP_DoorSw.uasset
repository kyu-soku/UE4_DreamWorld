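; BP_DoorSw is a pressure switch that controls a linked Door.
; Trigger overlap plays the ONOFF timeline to sink the Switch mesh, acting on the Door once fully pressed, and reverses it on exit.
; Flags pick the mode: OpenOnly opens once, HoldDown closes on release, Save opens once and registers the door with BP_GameInstance, and otherwise a FlipFlop toggles it.
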(event `self.Trigger.OnComponentBeginOverlap`
  (params (OverlappedComponent :type "PrimitiveComponent Object Reference") (OtherActor :type "Actor Object Reference") (OtherComp :type "PrimitiveComponent Object Reference") (OtherBodyIndex :type Integer) (bFromSweep :type Boolean) (SweepResult :type "HitResult Structure (by ref)"))
  (bind (_direction _onoff) (`Timeline|ONOFF` :!label _label)
    (:`Update`
      (`SceneComponent.K2_SetRelativeLocation` (`self.Switch`) (`KismetMathLibrary.VLerp` (0.0 0.0 0.0) (0.0 0.0 -15.0) _onoff) false false))
    (:`Finished`
      (if (== _onoff 1.0)
        (if (`self.OpenOnly`)
          (`/Engine/EditorBlueprintResources/StandardMacros.DoOnce` false
            (:`Completed`
              (`/Game/Workbench/BliePrint/1F/BP_Door.Open` (`self.Door`) :!label _label_2)))
          (elif (`self.HoldDown`)
            (goto _label_2)
            (elif (`self.Save`)
              (`self.DoOnceChangeDoor`)
              (else
                (`self.ChangeDoor`)))))))))

(event `self.Trigger.OnComponentEndOverlap`
  (params (OverlappedComponent :type "PrimitiveComponent Object Reference") (OtherActor :type "Actor Object Reference") (OtherComp :type "PrimitiveComponent Object Reference") (OtherBodyIndex :type Integer))
  (if (`self.HoldDown`)
    (`/Game/Workbench/BliePrint/1F/BP_Door.Close` (`self.Door`))
    (goto _label :!via `Reverse`)
    (else
      (goto _label :!via `Reverse`))))

(event `ChangeDoor`
  (bind _door (`self.Door`))
  (`/Engine/EditorBlueprintResources/StandardMacros.FlipFlop`
    (:`A`
      (`/Game/Workbench/BliePrint/1F/BP_Door.Open` _door))
    (:`B`
      (`/Game/Workbench/BliePrint/1F/BP_Door.Close` _door))))

(event `DoOnceChangeDoor`
  (bind _door (`self.Door`))
  (`/Engine/EditorBlueprintResources/StandardMacros.DoOnce` false
    (:`Completed`
      (`/Game/Workbench/BliePrint/1F/BP_Door.Open` _door)
      (`/Game/Workbench/BP_GameInstance.SetSaveDoor` (cast `/Game/Workbench/BP_GameInstance` (`GameplayStatics.GetGameInstance`) :!pure true) _door))))

(fn `UserConstructionScript`)