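; BP_JumpCountUp is a one-shot pickup actor that modifies the player character's jumping ability.
; When the player pawn overlaps its Trigger component, the JumpZVelecity flag selects whether to overwrite the movement component's JumpZVelocity or the character's JumpMaxCount.
; Both values come from the pickup's own variables and replace the current ones rather than adding to them.
; The actor then destroys itself.
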(event `self.Trigger.OnComponentBeginOverlap`
  (params (OverlappedComponent :type "PrimitiveComponent Object Reference") (OtherActor :type "Actor Object Reference") (OtherComp :type "PrimitiveComponent Object Reference") (OtherBodyIndex :type Integer) (bFromSweep :type Boolean) (SweepResult :type "HitResult Structure (by ref)"))
  (bind _returnvalue (`GameplayStatics.GetPlayerPawn` 0))
  (bind _ascharacter (cast `Character` _returnvalue :!pure true))
  (if (== OtherActor _returnvalue)
    (if (`self.JumpZVelecity`)
      (set `CharacterMovementComponent.JumpZVelocity` (`self.Jump Z Velocity`) (`Character.CharacterMovement` _ascharacter))
      (else
        (set `Character.JumpMaxCount` (`self.Jump Max Count`) _ascharacter)))
    (`self.K2_DestroyActor`)))

(fn `UserConstructionScript`)