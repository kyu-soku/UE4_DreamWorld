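; BP_Needle is a needle trap actor that damages the player pawn when it overlaps the damage trigger.
; The externally callable MoveNeedle event plays a timeline that raises the needle and records its height.
; MoveBeside waits briefly, then slides the needle and NeedleBox sideways by a configurable distance over a configurable time, using the recorded height to keep the needle raised.
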(event `MoveNeedle(OnlyONe)`
  (bind (_direction _move) (`Timeline|Move(OnlyONe)`)
    (:`Update`
      (bind _returnvalue (`KismetMathLibrary.Lerp` 0.0 150.0 _move))
      (`SceneComponent.K2_SetRelativeLocation` (`self.Needle`) (`KismetMathLibrary.MakeVector` 0.0 0.0 _returnvalue) false false)
      (set `self.NeedleLocationZ` _returnvalue))))

(event `MoveBeside`
  (`KismetSystemLibrary.Delay` 1.0)
  (`TimelineComponent.SetPlayRate` (`self.Beside`) (/ 1.0 (`self.MoveBesideTime`)))
  (bind (_direction _beside) (`Timeline|Beside`)
    (:`Update`
      (bind _returnvalue (`KismetMathLibrary.Lerp` 0.0 (`self.BesideDistance(X)`) _beside))
      (`SceneComponent.K2_SetRelativeLocation` (`self.Needle`) (`KismetMathLibrary.MakeVector` _returnvalue 0.0 (`self.NeedleLocationZ`)) false false)
      (`SceneComponent.K2_SetRelativeLocation` (`self.NeedleBox`) (`KismetMathLibrary.MakeVector` _returnvalue 0.0 75.0) false false))))

(event `self.DamegeTrigger.OnComponentBeginOverlap`
  (params (OverlappedComponent :type "PrimitiveComponent Object Reference") (OtherActor :type "Actor Object Reference") (OtherComp :type "PrimitiveComponent Object Reference") (OtherBodyIndex :type Integer) (bFromSweep :type Boolean) (SweepResult :type "HitResult Structure (by ref)"))
  (if (== OtherActor (`GameplayStatics.GetPlayerPawn` 0))
    (`GameplayStatics.ApplyDamage` OtherActor 100.0)))

(fn `UserConstructionScript`)