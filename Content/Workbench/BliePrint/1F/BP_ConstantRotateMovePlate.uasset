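; Moving plate actor that shifts its Plate component along a two-axis path, apparently a loop judging by its names, without changing its rotation.
; On BeginPlay, XYRotate selects either the XYRotation timeline for horizontal XY motion or UpDown for vertical XZ motion.
; Play rate is the inverse of RoundTripTime, and timeline curves drive Lerps that span Distance, from zero on X and centered on the second axis.
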(event `self.ReceiveBeginPlay`
  (bind _distance (`self.Distance`))
  (bind _distance_2 (`self.Distance`))
  (bind _returnvalue (/ _distance_2 2.0))
  (bind _returnvalue_2 (/ _distance 2.0))
  ;[1 1 1] 上下移動
  (if (`self.XYRotate`)
    (`TimelineComponent.SetPlayRate` (`self.XYRotation`) (/ 1.0 (`self.RoundTripTime`)))
    (bind (_direction _directionx _directiony) (`Timeline|XYRotation`)
      (:`Update`
        (`SceneComponent.K2_SetRelativeLocation` (`self.Plate`) (`KismetMathLibrary.MakeVector` (`KismetMathLibrary.Lerp` 0.0 _distance _directionx) (`KismetMathLibrary.Lerp` (* _returnvalue_2 -1.0) _returnvalue_2 _directiony)) false false)))
    (else
      (`TimelineComponent.SetPlayRate` (`self.UpDown`) (/ 1.0 (`self.RoundTripTime`)))
      (bind (_direction_2 _directionx_2 _directionz) (`Timeline|UpDown`)
        (:`Update`
          (`SceneComponent.K2_SetRelativeLocation` (`self.Plate`) (`KismetMathLibrary.MakeVector` (`KismetMathLibrary.Lerp` 0.0 _distance_2 _directionx_2) 0.0 (`KismetMathLibrary.Lerp` (* _returnvalue -1.0) _returnvalue _directionz)) false false))))))

(fn `UserConstructionScript`)