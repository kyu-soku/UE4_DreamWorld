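; BP_UpDoor is a door that slides upward once every actor in its PlateTrigger array has been destroyed.
; On BeginPlay it binds to the OnDestroyed event of those trigger actors and increments a counter each time one fires.
; When the count equals the array length, the OpenDoor timeline plays and lerps the Door component's relative Z location to raise it.
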(event `self.ReceiveBeginPlay`
  (add `self.OnDestroyed` (`self.PlateTrigger`) (delegate `DestroyEvent`)))

(event `DestroyEvent` :!signature `self.OnDestroyed`
  (params (DestroyedActor :type "Actor Object Reference"))
  (bind _result (`/Engine/EditorBlueprintResources/StandardMacros.IncrementInt` (`self.Count`))
    (:`  `
      (bind _output_get (set `self.Count` _result))
      (if (== _output_get (`KismetArrayLibrary.Array_Length` (`self.PlateTrigger`)))
        (bind (_direction `_新規track_0`) (`Timeline|OpenDoor`)
          (:`Update`
            (`SceneComponent.K2_SetRelativeLocation` (`self.Door`) (`KismetMathLibrary.MakeVector` 0.0 0.0 (`KismetMathLibrary.Lerp` 0.0 200.0 `_新規track_0`)) false false)))))))

(fn `UserConstructionScript`)