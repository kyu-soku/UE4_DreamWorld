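; BP_NextStageWarp is an interactable warp that moves the player on to the next stage.
; On HasInteracted it disables player movement, spawns a warp particle effect and pauses briefly.
; If LastStage is set, it shows the game instance's last-stage loading display and opens the End level.
; Otherwise it waits out the loading display, increments the game instance's stage number and opens LevelName suffixed with that number.
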(event `/Game/Workbench/BliePrint/1F/BPI_Interact.HasInteracted`
  (bind _asbp_game_instance (cast `/Game/Workbench/BP_GameInstance` (`GameplayStatics.GetGameInstance`) :!pure true))
  (`CharacterMovementComponent.DisableMovement` (`Character.CharacterMovement` (cast `Character` (`GameplayStatics.GetPlayerPawn` 0) :!pure true)))
  (`GameplayStatics.SpawnEmitterAtLocation` "/Game/Workbench/Particle/P_Warp.P_Warp" (`SceneComponent.K2_GetComponentLocation` (`self.DefaultSceneRoot`)))
  (`KismetSystemLibrary.Delay` 1.0)
  (if (`self.LastStage`)
    (`/Game/Workbench/BP_GameInstance.LoadingDisplay(LastStage)` _asbp_game_instance)
    (`KismetSystemLibrary.Delay` 1.0)
    (`GameplayStatics.OpenLevel` "End")
    (else
      (bind _loadingtime (`/Game/Workbench/BP_GameInstance.LoadingDisplay` _asbp_game_instance))
      (`KismetSystemLibrary.Delay` _loadingtime)
      (bind _result (`/Engine/EditorBlueprintResources/StandardMacros.IncrementInt` (`/Game/Workbench/BP_GameInstance.StageNum` _asbp_game_instance (`/Game/Workbench/BP_GameInstance.Stage` _asbp_game_instance)))
        (:`  `
          (`GameplayStatics.OpenLevel` (`KismetStringLibrary.Conv_StringToName` (`KismetStringLibrary.JoinStringArray` (`|MakeArray` (`KismetStringLibrary.Conv_NameToString` (`self.Level Name`)) (`KismetStringLibrary.Conv_IntToString` _result)) ""))))))))

(fn `UserConstructionScript`)